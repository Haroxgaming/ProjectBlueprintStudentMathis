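; BP_Chest is an interactable chest that opens only after at least two keys have been collected through its Morekey event, which increments a counter.
; On Interact it reveals two key meshes and runs chained timelines that slide them forward, then turn them.
; The keys then hide, and after a short delay a final timeline rotates the lid open.
; Animations are offset from key transforms cached at BeginPlay.
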(event `self.ReceiveBeginPlay`
  (set `self.relative rotation` (`SceneComponent.RelativeRotation` (`self.Key1`)))
  (set `self.relative Location Key1` (`SceneComponent.RelativeLocation` (`self.Key1`)))
  (set `self.relative Location Key2` (`SceneComponent.RelativeLocation` (`self.Key2`))))

(event `More key`
  ;[1 1 1] Get key
  (`/Engine/EditorBlueprintResources/StandardMacros.IncrementInt` (`self.Key number`)))

(event `/Game/FirstPerson/Player/BPI_Interaction.Interact`
  (bind (_relative_rotation_roll _relative_rotation_pitch _relative_rotation_yaw) (`KismetMathLibrary.BreakRotator` (`self.relative rotation`)))
  (bind (_relative_location_key1_x _relative_location_key1_y _relative_location_key1_z) (`KismetMathLibrary.BreakVector` (`self.relative Location Key1`)))
  (bind (_relative_location_key2_x _relative_location_key2_y _relative_location_key2_z) (`KismetMathLibrary.BreakVector` (`self.relative Location Key2`)))
  ;[1 0.9466 0.4812] Open chest event
  (if (>= (`self.Key number`) 2)
    (`SceneComponent.SetVisibility` (`self.Key2`) true false)
    (`SceneComponent.SetVisibility` (`self.Key1`) true false)
    ;;[1 1 1] Location timeline
    (bind (_direction _key_forward) (`Timeline|Key`)
      (:`Update`
        (bind _returnvalue (* _key_forward -20.0))
        (`SceneComponent.K2_SetRelativeLocation` (`self.Key1`) (`KismetMathLibrary.MakeVector` _relative_location_key1_x (+ _relative_location_key1_y _returnvalue) _relative_location_key1_z) false false)
        (`SceneComponent.K2_SetRelativeLocation` (`self.Key2`) (`KismetMathLibrary.MakeVector` _relative_location_key2_x (+ _relative_location_key2_y _returnvalue) _relative_location_key2_z) false false))
      (:`Finished`
        ;;[1 1 1] Rotation timeline
        (bind (_direction_2 _rotate) (`Timeline|rotate key`)
          (:`Update`
            (`SceneComponent.K2_SetRelativeRotation` (`self.Key2`) (`KismetMathLibrary.MakeRotator` _relative_rotation_roll (- _relative_rotation_pitch (* _rotate (`self.AngleRotationkey`))) _relative_rotation_yaw) false false)
            (`SceneComponent.K2_SetRelativeRotation` (`self.Key1`) (`KismetMathLibrary.MakeRotator` _relative_rotation_roll (- _relative_rotation_pitch (* _rotate (`self.AngleRotationkey`))) _relative_rotation_yaw) false false))
          (:`Finished`
            ;;[1 1 1] Chest open
            (`SceneComponent.SetVisibility` (`self.Key2`) false false)
            (`SceneComponent.SetVisibility` (`self.Key1`) false false)
            (`KismetSystemLibrary.Delay` 0.5)
            (bind (_direction_3 _open) (`Timeline|Timeline`)
              (:`Update`
                (`SceneComponent.K2_SetRelativeRotation` (`self.Chest upper`) (`KismetMathLibrary.MakeRotator` (* (* _open (`self.AngleRotationCoffre`)) -1.0)) false false)))))))))

(fn `UserConstructionScript`)