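; BP_Door is a double door that swings open or closed when interacted with, unless it is flagged as locked.
; The Interact event drives a FlipFlop that alternates between playing and reversing a Timeline.
; The Timeline's Open track scales AngleRotation to set both leaves' relative yaw, with the right leaf mirrored from a 180-degree base.
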(event `/Game/FirstPerson/Player/BPI_Interaction.Interact`
  (if (not (`self.locked door`))
    (`/Engine/EditorBlueprintResources/StandardMacros.FlipFlop`
      (:`A`
        (bind (_direction _open) (`Timeline|Timeline` :!label _label)
          (:`Update`
            (bind _returnvalue (* _open (`self.AngleRotation`)))
            (`SceneComponent.K2_SetRelativeRotation` (`self.LeftDoor`) (`KismetMathLibrary.MakeRotator` 0.0 0.0 _returnvalue) false false)
            (`SceneComponent.K2_SetRelativeRotation` (`self.RightDoor`) (`KismetMathLibrary.MakeRotator` 0.0 0.0 (* (+ 180.0 _returnvalue) -1.0)) false false))))
      (:`B`
        (goto _label :!via `Reverse`)))))

(fn `UserConstructionScript`)